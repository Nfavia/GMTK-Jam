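; Base enemy Blueprint that supplies a WingFlap function for animating a pair of wings procedurally, with no active event logic of its own.
; Each call uses FInterpTo at WingFlapRate to roll the two wing components in opposite directions toward MaxFlapRotation, or back toward zero.
; The ReverseFlap flag toggles once both wings are within five degrees of the target, so repeated calls produce a continuous flap cycle.
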(fn `UserConstructionScript`)

(fn `WingFlap`
  (params (WingLeft :type "StaticMeshComponent Object Reference") (WingRight :type "StaticMeshComponent Object Reference") (DeltaTime :type "Float (double-precision)"))
  (bind _wingleft (`local.WingLeft`))
  (bind _wingright (`local.WingRight`))
  (bind _wingleft_2 (`local.WingLeft`))
  (bind _wingright_2 (`local.WingRight`))
  (bind (_relativerotation_roll _relativerotation_pitch _relativerotation_yaw) (`KismetMathLibrary.BreakRotator` (`SceneComponent.RelativeRotation` _wingleft_2)))
  (bind _relativerotation_roll_2 (`KismetMathLibrary.BreakRotator` (`SceneComponent.RelativeRotation` _wingright)))
  (bind _relativerotation_roll_3 (`KismetMathLibrary.BreakRotator` (`SceneComponent.RelativeRotation` _wingleft)))
  (bind (_relativerotation_roll_4 _relativerotation_pitch_2 _relativerotation_yaw_2) (`KismetMathLibrary.BreakRotator` (`SceneComponent.RelativeRotation` _wingleft)))
  (bind (_relativerotation_roll_5 _relativerotation_pitch_3) (`KismetMathLibrary.BreakRotator` (`SceneComponent.RelativeRotation` _wingright)))
  (bind _relativerotation_roll_6 (`KismetMathLibrary.BreakRotator` (`SceneComponent.RelativeRotation` _wingright_2)))
  (bind _relativerotation_roll_7 (`KismetMathLibrary.BreakRotator` (`SceneComponent.RelativeRotation` _wingleft_2)))
  (bind (_relativerotation_roll_8 _relativerotation_pitch_4) (`KismetMathLibrary.BreakRotator` (`SceneComponent.RelativeRotation` _wingright_2)))
  (`/Engine/EditorBlueprintResources/StandardMacros.IsValid` WingLeft
    (:`Is Valid`
      (`/Engine/EditorBlueprintResources/StandardMacros.IsValid` WingRight
        (:`Is Valid`
          (if (`self.ReverseFlap`)
            (`|ExecutionSequence`
              (:`then_0`
                (`SceneComponent.K2_SetRelativeRotation` _wingright_2 (`KismetMathLibrary.MakeRotator` (`KismetMathLibrary.FInterpTo` _relativerotation_roll_8 0.0 (`local.DeltaTime`) (`self.WingFlapRate`)) _relativerotation_pitch_4) false false))
              (:`then_1`
                (`SceneComponent.K2_SetRelativeRotation` _wingleft_2 (`KismetMathLibrary.MakeRotator` (`KismetMathLibrary.FInterpTo` _relativerotation_roll 0.0 (`local.DeltaTime`) (`self.WingFlapRate`)) _relativerotation_pitch _relativerotation_yaw) false false)))
            (if (and (<= _relativerotation_roll_6 5.0) (>= _relativerotation_roll_7 -5.0))
              (set `self.ReverseFlap` false))
            (else
              (`|ExecutionSequence`
                (:`then_0`
                  (`SceneComponent.K2_SetRelativeRotation` _wingright (`KismetMathLibrary.MakeRotator` (`KismetMathLibrary.FInterpTo` _relativerotation_roll_5 (`self.MaxFlapRotation`) (`local.DeltaTime`) (`self.WingFlapRate`)) _relativerotation_pitch_3) false false))
                (:`then_1`
                  (`SceneComponent.K2_SetRelativeRotation` _wingleft (`KismetMathLibrary.MakeRotator` (`KismetMathLibrary.FInterpTo` _relativerotation_roll_4 (* (`self.MaxFlapRotation`) -1.0) (`local.DeltaTime`) (`self.WingFlapRate`)) _relativerotation_pitch_2 _relativerotation_yaw_2) false false)))
              (if (and (>= _relativerotation_roll_2 (- (`self.MaxFlapRotation`) 5.0)) (<= _relativerotation_roll_3 (+ (* (`self.MaxFlapRotation`) -1.0) 5.0)))
                (set `self.ReverseFlap` true)))))))))