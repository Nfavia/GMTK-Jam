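; Teeter stack actor, in an OLD folder, that piles overlapping stackable objects into a physics-driven tower on its base.
; StackDetector overlaps feed AddItemToStack, which attaches each item, snaps it above the previous one and stops at a maximum index.
; The bottom item stays non-simulated, while later items simulate physics, linked by six pre-placed constraints moved to item top points.
; Other functions total item count and size-based score, or clear constraints and destroy the stack.
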(event `self.ReceiveBeginPlay`
  ;[0.1352 0.8702 1] Begin Play
  (`self.InitializeStack`))

(event `self.StackDetector.OnComponentBeginOverlap`
  (params (OverlappedComponent :type "PrimitiveComponent Object Reference") (OtherActor :type "Actor Object Reference") (OtherComp :type "PrimitiveComponent Object Reference") (OtherBodyIndex :type Integer) (bFromSweep :type Boolean) (SweepResult :type "HitResult Structure (by ref)"))
  (bind _asstackable_object_base (cast `/Game/Blueprints/StackableObjects/Testing/StackableObjectBase` OtherActor))
  (if (`/Game/Blueprints/StackableObjects/Testing/StackableObjectBase.CanBeStacked` _asstackable_object_base)
    (`self.AddItemToStack` _asstackable_object_base)))

(fn `AddItemToStack`
  (params (NewItem :type "/Game/Blueprints/StackableObjects/Testing/StackableObjectBase Object Reference"))
  (locals (NewItemTop :type "Float (double-precision)" :default 0.0))
  (bind _newstackitem (`self.NewStackItem`))
  (bind _body (`/Game/Blueprints/StackableObjects/Testing/StackableObjectBase.Body` (`self.NewStackItem`)))
  (bind _output_get (set `self.NewStackItem` NewItem))
  (`/Engine/EditorBlueprintResources/StandardMacros.IsValid` _output_get
    (:`Is Valid`
      (if (`self.CanStack`)
        (`|ExecutionSequence`
          (:`then_0`
            ;[1 1 1] Setup Stack Item and attach to base or last stack Item
            (`PrimitiveComponent.SetSimulatePhysics` _body false)
            (`PrimitiveComponent.SetLinearDamping` _body 0.5)
            (`self.K2_AttachToActor` (`self.NewStackItem`) self "None" "SnapToTarget" "SnapToTarget" "KeepWorld" true)
            (set `/Game/Blueprints/StackableObjects/Testing/StackableObjectBase.InStack` true _newstackitem)
            (`KismetArrayLibrary.Array_Add` (`self.StackItems`) _newstackitem))
          (:`then_1`
            ;[1 0.4081 0.688] Check if this is the base
            (if (== (`self.CurrentStackIndex`) 0)
              ;[1 1 1] Attached to Base
              (`self.K2_SetActorLocation` (`self.NewStackItem`) (+ (`SceneComponent.K2_GetComponentLocation` (`self.Base`)) (`KismetMathLibrary.MakeVector` 0.0 0.0 (.z (`.BoxExtent` (`KismetSystemLibrary.GetComponentBounds` (`/Game/Blueprints/StackableObjects/Testing/StackableObjectBase.Body` (`self.NewStackItem`))))))) false false)
              (else
                ;[1 1 1] Set location to on top of last item
                (`self.K2_SetActorLocation` (`self.NewStackItem`) (+ (`SceneComponent.K2_GetComponentLocation` (`/Game/Blueprints/StackableObjects/Testing/StackableObjectBase.TopPoint` (`self.LastStackItem`))) (`KismetMathLibrary.MakeVector` 0.0 0.0 (+ (.z (`.BoxExtent` (`KismetSystemLibrary.GetComponentBounds` (`/Game/Blueprints/StackableObjects/Testing/StackableObjectBase.Body` (`self.NewStackItem`))))) (`self.VerticalOffset`)))) false false))))
          (:`then_2`
            ;[1 1 1] Setup Constraints
            (`SceneComponent.K2_SetWorldLocation` (`|GetArrayItem` (`self.Constraints`) (`self.CurrentStackIndex`)) (`SceneComponent.K2_GetComponentLocation` (`/Game/Blueprints/StackableObjects/Testing/StackableObjectBase.TopPoint` (`self.NewStackItem`))) false false)
            ;;[1 0.4263 0.707] Dont set constraints on first item in stack
            (if (not (== (`self.CurrentStackIndex`) 0))
              (`PhysicsConstraintComponent.SetConstrainedComponents` (`|GetArrayItem` (`self.Constraints`) (- (`self.CurrentStackIndex`) 1)) (`/Game/Blueprints/StackableObjects/Testing/StackableObjectBase.Body` (`self.LastStackItem`)) "None" (`/Game/Blueprints/StackableObjects/Testing/StackableObjectBase.Body` (`self.NewStackItem`)) "None")))
          (:`then_3`
            ;[1 1 1] Cleanup and increment
            ;;[1 0.3897 0.6688] Only Simulate Physics if it isn't the base
            (if (not (== (`self.CurrentStackIndex`) 0))
              (`PrimitiveComponent.SetSimulatePhysics` (`/Game/Blueprints/StackableObjects/Testing/StackableObjectBase.Body` (`self.NewStackItem`)) true))
            (set `self.LastStackItem` (`self.NewStackItem`))
            (set `self.NewStackItem` null)
            (if (>= (`self.CurrentStackIndex`) (`self.MaxStackIndex`))
              (set `self.CanStack` false)
              (else
                (`/Engine/EditorBlueprintResources/StandardMacros.IncrementInt` (`self.CurrentStackIndex`))))))))))

(fn `Check Items Within Stack`
  (returns (NumberItemsInStack :type Integer) (TotalScoreWithinStack :type Integer))
  (bind _stackitems (`self.StackItems`))
  (bind _totalstacksizevalue (`self.TotalStackSizeValue`))
  (for _array_element _stackitems
    (set `self.TotalStackSizeValue` (+ (`/Game/Blueprints/StackableObjects/Testing/StackableObjectBase.SizeValue` _array_element) _totalstacksizevalue)))
  (return (`KismetArrayLibrary.Array_Length` _stackitems) _totalstacksizevalue))

(fn `InitializeStack`
  (locals (Temp :type Boolean :default true))
  (`|ExecutionSequence`
    (:`then_0`
      ;[1 0.2809 0.7427] Setup Stack variables
      (set `self.CurrentStackIndex` 0)
      ;;[1 0.7149 0.3122] Make Array of Constraints
      (set `self.Constraints` (`|MakeArray` (`self.PhysicsConstraint0`) (`self.PhysicsConstraint1`) (`self.PhysicsConstraint2`) (`self.PhysicsConstraint3`) (`self.PhysicsConstraint4`) (`self.PhysicsConstraint5`)))
      (set `self.CanStack` true))
    (:`then_1`
      ;[1 0.3008 0.2809] Setup Stack Detector
      (`SceneComponent.K2_SetWorldLocation` (`self.StackDetector`) (`SceneComponent.K2_GetComponentLocation` (`self.Base`)) false false))))

(fn `MoveStackUp`)

(fn `Remove All Items From Stack`
  (bind _stackitems (`self.StackItems`))
  ;[1 1 1] Remove Constraints
  (for _array_element (`self.Constraints`)
    (`PhysicsConstraintComponent.SetConstrainedComponents` _array_element null "None" null "None"))
  ;[1 1 1] Destroy Actors In Stack
  (for _array_element_2 _stackitems
    (`self.K2_DestroyActor` _array_element_2)
    (`KismetSystemLibrary.PrintString` (`KismetSystemLibrary.GetDisplayName` _array_element_2)))
  ;[1 1 1] Cleanup Variables
  (`KismetArrayLibrary.Array_Clear` _stackitems)
  (set `self.CurrentStackIndex` 0)
  (set `self.CanStack` true)
  (return))

(fn `UserConstructionScript`)