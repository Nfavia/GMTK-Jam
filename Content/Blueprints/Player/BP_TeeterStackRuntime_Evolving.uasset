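; Runtime Blueprint for a player's teetering stack of physics items, built upward from a Base component.
; Each added item snaps above the previous item's TopPoint; the first stays non-simulated, while later ones simulate physics, linked by a pool of six pre-placed constraints.
; Stacking stops at MaxStack, and helpers total item size values or clear the constraints.
; MoveStackUp is an empty stub, and StackDetector collision is disabled on BeginPlay.
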(event `self.ReceiveBeginPlay`
  ;[0.1352 0.8702 1] Begin Play
  (`self.InitializeStack`))

(fn `AddItemToStack`
  (params (NewItem :type "/Game/Blueprints/StackableObjectBase Object Reference"))
  (locals (NewItemTop :type "Float (double-precision)" :default 0.0))
  (bind _newstackitem (`self.NewStackItem`))
  (bind _body (`/Game/Blueprints/StackableObjectBase.Body` (`self.NewStackItem`)))
  (bind _output_get (set `self.NewStackItem` NewItem))
  (`/Engine/EditorBlueprintResources/StandardMacros.IsValid` _output_get
    (:`Is Valid`
      (if (`self.CanStack`)
        (`|ExecutionSequence`
          (:`then_0`
            ;[1 1 1] Setup Stack Item and attach
            (`PrimitiveComponent.SetSimulatePhysics` _body false)
            (`PrimitiveComponent.SetLinearDamping` _body 0.5)
            (`self.K2_AttachToComponent` (`self.NewStackItem`) (`self.Base`) "None" "SnapToTarget" "KeepRelative" "KeepWorld" true))
          (:`then_1`
            ;[1 1 1] Check if this is the base
            (if (== (`self.CurrentStackIndex`) 0)
              ;[1 1 1] Attached to Base
              (`self.K2_SetActorLocation` (`self.NewStackItem`) (+ (`SceneComponent.K2_GetComponentLocation` (`self.Base`)) (`KismetMathLibrary.MakeVector` 0.0 0.0 (/ (`.SphereRadius` (`KismetSystemLibrary.GetComponentBounds` (`/Game/Blueprints/StackableObjectBase.Body` (`self.NewStackItem`)))) 1.5))) false false)
              (else
                ;[1 1 1] Set location to on top of last item
                (`self.K2_SetActorLocation` (`self.NewStackItem`) (+ (`SceneComponent.K2_GetComponentLocation` (`/Game/Blueprints/StackableObjectBase.TopPoint` (`self.LastStackItem`))) (`KismetMathLibrary.MakeVector` 0.0 0.0 (+ (/ (`.SphereRadius` (`KismetSystemLibrary.GetComponentBounds` (`/Game/Blueprints/StackableObjectBase.Body` (`self.NewStackItem`)))) 1.5) 1.0))) false false))))
          (:`then_2`
            ;[1 1 1] Setup Constraints
            (`SceneComponent.K2_SetWorldLocation` (`|GetArrayItem` (`self.Constraints`) (`self.CurrentStackIndex`)) (`SceneComponent.K2_GetComponentLocation` (`/Game/Blueprints/StackableObjectBase.TopPoint` (`self.NewStackItem`))) false false)
            ;;[1 1 1] Dont set constraints on first item in stack
            (if (not (== (`self.CurrentStackIndex`) 0))
              (`PhysicsConstraintComponent.SetConstrainedComponents` (`|GetArrayItem` (`self.Constraints`) (- (`self.CurrentStackIndex`) 1)) (`/Game/Blueprints/StackableObjectBase.Body` (`self.LastStackItem`)) "None" (`/Game/Blueprints/StackableObjectBase.Body` (`self.NewStackItem`)) "None")))
          (:`then_3`
            ;[1 1 1] Cleanup and increment
            (if (not (== (`self.CurrentStackIndex`) 0))
              (`PrimitiveComponent.SetSimulatePhysics` (`/Game/Blueprints/StackableObjectBase.Body` (`self.NewStackItem`)) true))
            (set `self.LastStackItem` _newstackitem)
            (`KismetArrayLibrary.Array_Add` (`self.StackItems`) _newstackitem)
            (set `self.NewStackItem` null)
            (bind _result (`/Engine/EditorBlueprintResources/StandardMacros.IncrementInt` (`self.CurrentStackIndex`))
              (:`  `
                (if (>= _result (`self.MaxStack`))
                  (set `self.CanStack` false))))))))))

(fn `Check items within stack`
  (returns (NumberItemsInStack :type Integer) (TotalScoreWithinStack :type Integer))
  (bind _stackitems (`self.StackItems`))
  (bind _totalstacksizevalue (`self.TotalStackSizeValue`))
  (for _array_element _stackitems
    (set `self.TotalStackSizeValue` (+ (`/Game/Blueprints/StackableObjectBase.SizeValue` _array_element) _totalstacksizevalue)))
  (return (`KismetArrayLibrary.Array_Length` _stackitems) _totalstacksizevalue))

(fn `InitializeStack`
  (locals (Temp :type Boolean :default true))
  (bind _stackdetector (`self.StackDetector`))
  (`|ExecutionSequence`
    (:`then_0`
      ;[1 0.2809 0.7427] Setup Stack variables
      (set `self.CurrentStackIndex` 0)
      ;;[1 0.7149 0.3122] Make Array of Constraints
      (set `self.Constraints` (`|MakeArray` (`self.PhysicsConstraint0`) (`self.PhysicsConstraint1`) (`self.PhysicsConstraint2`) (`self.PhysicsConstraint3`) (`self.PhysicsConstraint4`) (`self.PhysicsConstraint5`)))
      (set `self.CanStack` true))
    (:`then_1`
      ;[1 0.3008 0.2809] Setup Stack Detector
      (`SceneComponent.K2_SetWorldLocation` _stackdetector (`SceneComponent.K2_GetComponentLocation` (`self.Base`)) false false)
      (`PrimitiveComponent.SetCollisionEnabled` _stackdetector "NoCollision"))))

(fn `MoveStackUp`)

(fn `RemoveItemsFromStack`
  (for _array_element (`self.Constraints`)
    (`PhysicsConstraintComponent.SetConstrainedComponents` _array_element null "None" null "None")))

(fn `UserConstructionScript`)