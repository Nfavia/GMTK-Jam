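; GrowthPond is a trigger actor that marks when an evolving turtle is inside a growth pond.
; On begin and end overlap it checks whether the other actor derives from TESTING_EvolvingTurtle, casts it, and sets its IsInGrowthPond flag true or false.
; Begin overlap also prints a debug message for any overlapping actor; the pond holds no growth logic itself.
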(event `self.ReceiveActorBeginOverlap`
  (params (OtherActor :type "Actor Object Reference"))
  (`KismetSystemLibrary.PrintString` "object is overlapping")
  (if (`KismetMathLibrary.ClassIsChildOf` (`GameplayStatics.GetObjectClass` OtherActor) "/Game/Blueprints/Player/TESTING_EvolvingTurtle.TESTING_EvolvingTurtle_C")
    (bind _astesting_evolving_turtle (cast `/Game/Blueprints/Player/TESTING_EvolvingTurtle` OtherActor))
    (set `/Game/Blueprints/Player/TESTING_EvolvingTurtle.IsInGrowthPond` true _astesting_evolving_turtle)))

(event `self.ReceiveActorEndOverlap`
  (params (OtherActor :type "Actor Object Reference"))
  (if (`KismetMathLibrary.ClassIsChildOf` (`GameplayStatics.GetObjectClass` OtherActor) "/Game/Blueprints/Player/TESTING_EvolvingTurtle.TESTING_EvolvingTurtle_C")
    (bind _astesting_evolving_turtle (cast `/Game/Blueprints/Player/TESTING_EvolvingTurtle` OtherActor))
    (set `/Game/Blueprints/Player/TESTING_EvolvingTurtle.IsInGrowthPond` false _astesting_evolving_turtle)))

(fn `UserConstructionScript`)